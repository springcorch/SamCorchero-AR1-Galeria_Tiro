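; BP_Floor is a floor that acts as the losing sequence once the game ends with too few points.
; Tick polls BP_GameManager and, while the game has ended below MinPoints, moves the Floor component along Z at Speed.
; Any actor overlap prints the losing score and point difference, destroys the Trigger to avoid repeats, then calls the manager's Restart after WaitRestart seconds.
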(event Collision|EventActorBeginOverlap
  (params (OtherActor :type Actor%20Object%20Reference))
  ;[0.75 0.1919 0.6221] Si colisiona con el jugador se muestra un mensaje, se destruye el trigger para evitar fallos y se espera unos segundos propuestos para después iniciar un evento del gamemanager que reiniciará la escena
  (bind _returnvalue (Actor|GetActorOfClass "/Game/CORREGIR/BP_GameManager.BP_GameManager_C"))
  (Development|PrintString (Utilities|String|Append "Has perdido con una puntuación de " (Utilities|String|ToString(Integer) (Variables|/Game/CORREGIR/BP_GameManager.BP_GameManager_C|GetTotalPoints _returnvalue)) ". Te han faltado " (Utilities|String|ToString(Integer) (- (Variables|/Game/CORREGIR/BP_GameManager.BP_GameManager_C|GetTotalPoints _returnvalue) (Variables|/Game/CORREGIR/BP_GameManager.BP_GameManager_C|GetminPoints _returnvalue))) " puntos para ganar.") true true "(R=1.000000,G=0.000000,B=0.000000,A=1.000000)" 1e+01)
  (Components|DestroyComponent (Variables|Default|Gettrigger))
  (Utilities|FlowControl|Delay (Variables|Default|GetwaitRestart))
  (bind _returnvalue_2 (Actor|GetActorOfClass "/Game/CORREGIR/BP_GameManager.BP_GameManager_C"))
  (Default|Restart _returnvalue_2))

(event EventTick
  (params (DeltaSeconds :type Float%20%28single-precision%29))
  ;[0.5174 0.2401 0.75] Se espera a que el juego haya terminado, si es así, se mueve infinitamente hacia abajo
  (bind _returnvalue (Actor|GetActorOfClass "/Game/CORREGIR/BP_GameManager.BP_GameManager_C"))
  (if (Variables|/Game/CORREGIR/BP_GameManager.BP_GameManager_C|GetgameEnded _returnvalue)
    (if (> (Variables|/Game/CORREGIR/BP_GameManager.BP_GameManager_C|GetminPoints _returnvalue) (Variables|/Game/CORREGIR/BP_GameManager.BP_GameManager_C|GetTotalPoints _returnvalue))
      (Transformation|AddWorldOffset (Variables|Default|GetFloor) (Math|Vector|MakeVector 0.0 0.0 (* DeltaSeconds (Variables|Default|Getspeed))) false false))))

(fn ConstructionScript)