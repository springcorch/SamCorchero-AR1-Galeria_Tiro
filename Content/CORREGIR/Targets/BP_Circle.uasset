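; BP_Circle is a moving target actor that travels sideways along world Y at a set Speed.
; On BeginPlay it finds BP_Spawner and copies its IsRight flag, which sets the direction of the per-frame, delta-time-scaled offset in Tick.
; A hit destroys both the other actor and the circle, while any actor overlap destroys only the circle.
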(event EventBeginPlay
  (bind _returnvalue (Actor|GetActorOfClass "/Game/CORREGIR/BP_Spawner.BP_Spawner_C"))
  (Variables|Default|SetgoRight (Variables|/Game/CORREGIR/BP_Spawner.BP_Spawner_C|GetIsRight _returnvalue)))

(event Collision|EventActorBeginOverlap
  (params (OtherActor :type Actor%20Object%20Reference))
  (Actor|DestroyActor))

(event EventTick
  (params (DeltaSeconds :type Float%20%28single-precision%29))
  (bind _speed (Variables|Default|Getspeed))
  (if (Variables|Default|GetgoRight)
    (Transformation|AddActorWorldOffset (Math|Vector|MakeVector 0.0 (* (* _speed 1.0) DeltaSeconds) 0.0))
    (else
      (Transformation|AddActorWorldOffset (Math|Vector|MakeVector 0.0 (* DeltaSeconds (* _speed -1.0)) 0.0)))))

(event Collision|EventHit
  (params (MyComp :type Primitive%20Component%20Object%20Reference) (Other :type Actor%20Object%20Reference) (OtherComp :type Primitive%20Component%20Object%20Reference) (bSelfMoved :type Boolean) (HitLocation :type Vector :default "0, 0, 0") (HitNormal :type Vector :default "0, 0, 0") (NormalImpulse :type Vector :default "0, 0, 0") (Hit :type Hit%20Result%20Structure%20%28by%20ref%29))
  (Actor|DestroyActor Other)
  (Actor|DestroyActor))

(fn ConstructionScript)