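; BP_Cone is a moving target or projectile that travels sideways along the Y axis and destroys itself on contact.
; On BeginPlay it finds the BP_Spawner and copies its IsRight flag to choose its direction.
; Tick offsets it by Speed scaled by delta time, negated for leftward movement.
; Any hit or actor overlap destroys it.
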(event EventBeginPlay
  ;[0.2664 0.2597 0.75] Al inciarse, obtiene la variable del spawner para saber en qué dirección ir
  (bind _returnvalue (Actor|GetActorOfClass "/Game/CORREGIR/BP_Spawner.BP_Spawner_C"))
  (Variables|Default|SetgoRight (Variables|/Game/CORREGIR/BP_Spawner.BP_Spawner_C|GetIsRight _returnvalue)))

(event Collision|EventActorBeginOverlap
  (params (OtherActor :type Actor%20Object%20Reference))
  ;[0.7466 0.4219 0.75] Cuando choca con un trigger se destruye a si mismo
  (Actor|DestroyActor))

(event EventTick
  (params (DeltaSeconds :type Float%20%28single-precision%29))
  (bind _speed (Variables|Default|Getspeed))
  ;[0.3661 0.75 0.6316] Uso un tick para que vaya hacía la dirección indicada smoothly, el branch decide si va hacia la derecha o izquierda (*-1)
  (if (Variables|Default|GetgoRight)
    (Transformation|AddActorWorldOffset (Math|Vector|MakeVector 0.0 (* _speed DeltaSeconds) 0.0))
    (else
      (Transformation|AddActorWorldOffset (Math|Vector|MakeVector 0.0 (* DeltaSeconds (* _speed -1.0)) 0.0)))))

(event Collision|EventHit
  (params (MyComp :type Primitive%20Component%20Object%20Reference) (Other :type Actor%20Object%20Reference) (OtherComp :type Primitive%20Component%20Object%20Reference) (bSelfMoved :type Boolean) (HitLocation :type Vector :default "0, 0, 0") (HitNormal :type Vector :default "0, 0, 0") (NormalImpulse :type Vector :default "0, 0, 0") (Hit :type Hit%20Result%20Structure%20%28by%20ref%29))
  ;[0.75 0.3758 0.278] Si choca contra un objeto se destruye (projectil)
  (Actor|DestroyActor))

(fn ConstructionScript)