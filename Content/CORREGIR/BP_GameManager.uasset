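; BP_GameManager runs a start-of-game countdown that ends with a "SHOOT!" message.
; BeginPlay resets CountDown to MaxCountDown.
; Each StartGame call prints and decrements CountDown; at zero it prints "SHOOT!" and pauses its timer by function name.
; The timer that drives StartGame is not started in this Blueprint's graphs.
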(event EventBeginPlay
  ;[0.4536 0.4233 1 0.75] Se inicia el contador a los segundos máximos al iniciar BP
  (Variables|Default|SetCountDown (Variables|Default|GetmaxCountDown)))

(event Collision|EventActorBeginOverlap
  (params (OtherActor :type Actor%20Object%20Reference)))

(event EventTick
  (params (DeltaSeconds :type Float%20%28single-precision%29)))

(fn ConstructionScript)

(fn StartGame
  ;[0.3808 0.3432 1 0.75] Cuando la variable haya llegado a 0, se mostrará que ya se puede jugar y acabará la función, si no, se restará a countDown por uno cada vez que se inicie la variable
  (if (== (Variables|Default|GetCountDown) 0)
    (Development|PrintString "SHOOT!" true true "(R=0.000000,G=0.660000,B=1.000000,A=1.000000)" 6.0)
    (Class|KismetSystemLibrary|PauseTimer 0 "Start Game")
    (else
      (Development|PrintString (Utilities|String|ToString(Integer) (Variables|Default|GetCountDown)) true true "(R=0.000000,G=0.660000,B=1.000000,A=1.000000)" 6.0)
      (Variables|Default|SetCountDown (- (Variables|Default|GetCountDown) 1)))))